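; Door component that moves a supplied hinge component between closed and open transforms and tracks the door's state.
; Setting the state alpha applies an ease-in-out blend to the hinge, then derives open, closed or intermediate state from thresholds.
; The state's RepNotify fires a state-changed dispatcher, and BeginPlay reports a missing hinge.
; Setting the state directly is unfinished and only prints a warning.
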(event EventBeginPlay
  (CallFunction|UpdateDoorState)
  (Variables|Default|GetDoorHinge
    (:then)
    (:else
      (Development|PrintString "Error: Door hinge not set!" true true "(R=1.000000,G=0.000000,B=0.000000,A=1.000000)"))))

(event EventTick
  (params (DeltaSeconds :type Float%20%28single-precision%29)))

(fn OnRepDoorState
  (Default|CallOnDoorStateChanged (Variables|Default|GetDoorState)))

(fn GetDoorState
  (return (Variables|Default|GetDoorState)))

(fn SetDoorState
  (params (DoorState :type E_DoorState%20Enum :default "NewEnumerator0"))
  (Development|PrintString "FINISH THIS! DOOR SHOULD ANIMATE TO THE CORRECT POSITION WHEN THIS IS SET MANUALLY!" true true "(R=1.000000,G=0.009744,B=0.000000,A=1.000000)" 5.0))

(fn GetDoorStateAlpha
  (return (Variables|Default|GetDoorStateAlpha)))

(fn SetDoorStateAlpha
  (params (DoorStateAlpha :type Float%20%28single-precision%29))
  (Variables|Default|SetDoorStateAlpha DoorStateAlpha)
  (Transformation|SetRelativeTransform (Variables|Default|GetDoorHinge) (Math|Interpolation|Ease "EaseInOut" (Variables|Default|GetDoorStateAlpha) (Variables|Default|GetInitialClosedTransformation) (Variables|Default|GetFinalOpenTransformation) 2.0) false false)
  (CallFunction|UpdateDoorState))

(fn SetDoorHinge
  (params (DoorHinge :type Scene%20Component%20Object%20Reference))
  (Variables|Default|SetDoorHinge DoorHinge))

(fn UpdateDoorState
  (Variables|Default|SetDoorState (select (>= (Variables|Default|GetDoorStateAlpha) (Variables|Default|GetOpenAlpha)) "NewEnumerator1" (select (<= (Variables|Default|GetDoorStateAlpha) (Variables|Default|GetClosedAlpha)) "NewEnumerator0" "NewEnumerator4"))))