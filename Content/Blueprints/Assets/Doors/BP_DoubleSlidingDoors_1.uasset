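; BP_DoubleSlidingDoors_1 is an interactable pair of doors that open and close together, with a state-based prompt at a marker component.
; Construction hands each side's door component its hinge and closed/open transforms taken from placed marker components.
; A single timeline plays or reverses to drive both components' state alpha.
; Interact and prompt text read only the left door's state, and Interact toggles only when fully open or closed.
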(event Custom|OpenDoor
  (bind _alpha (Timeline|DoorAlpha Play)
    (:Update
      (Class|COVDoorComponent|SetDoorStateAlpha (Variables|Default|GetLeftDoor_DoorComponent) _alpha)
      (Class|COVDoorComponent|SetDoorStateAlpha (Variables|Default|GetRightDoor_DoorComponent) _alpha))))

(event Custom|CloseDoor
  (bind _alpha (Timeline|DoorAlpha Reverse)
    (:Update
      (Class|COVDoorComponent|SetDoorStateAlpha (Variables|Default|GetLeftDoor_DoorComponent) _alpha)
      (Class|COVDoorComponent|SetDoorStateAlpha (Variables|Default|GetRightDoor_DoorComponent) _alpha))))

(event EventBeginPlay)

(event Collision|EventActorBeginOverlap
  (params (OtherActor :type Actor%20Object%20Reference)))

(event EventTick
  (params (DeltaSeconds :type Float%20%28single-precision%29)))

(fn ConstructionScript
  (Default|SetDoorHinge (Variables|Default|GetLeftDoor_DoorComponent) (Variables|Default|GetLeftDoorHinge))
  (Default|SetDoorHinge (Variables|Default|GetRightDoor_DoorComponent) (Variables|Default|GetRightDoorHinge))
  (Class|COVDoorComponent|SetInitialClosedTransform (Variables|Default|GetLeftDoor_DoorComponent) (Transformation|GetRelativeTransform (Variables|Default|GetClosedPositionLeft)))
  (Class|COVDoorComponent|SetInitialClosedTransform (Variables|Default|GetRightDoor_DoorComponent) (Transformation|GetRelativeTransform (Variables|Default|GetClosedPositionRight)))
  (Class|COVDoorComponent|SetFinalOpenTransform (Variables|Default|GetLeftDoor_DoorComponent) (Transformation|GetRelativeTransform (Variables|Default|GetOpenPositionLeft)))
  (Class|COVDoorComponent|SetFinalOpenTransform (Variables|Default|GetRightDoor_DoorComponent) (Transformation|GetRelativeTransform (Variables|Default|GetOpenPositionRight))))

(fn GetDefaultPromptLocation
  (return (Transformation|GetWorldLocation (Variables|Default|GetPromptLocation))))

(fn GetDefaultPromptText
  (return (Utilities|Select :Index (Class|COVDoorComponent|GetDoorState (Variables|Default|GetLeftDoor_DoorComponent)) :Closed "Open door" :Closing "Closing..." :Open "Close door" :Opening "Opening..." :Cracked "Cracked...")))

(fn GetIsInteractable
  (return true))

(fn Interact
  (params (Interactor :type Actor%20Object%20Reference))
  (switch Utilities|FlowControl|Switch|SwitchonEDoorState (Default|GetDoorState (Variables|Default|GetLeftDoor_DoorComponent))
    (:Closed
      (CallFunction|OpenDoor))
    (:Open
      (CallFunction|CloseDoor)))
  (return true))