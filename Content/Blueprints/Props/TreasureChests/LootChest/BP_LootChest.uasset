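; Loot chest prop that players interact with to open, and to close again when CanBeClosed allows it.
; Interact plays or reverses a timeline that sets the BPC_Door component's alpha between closed and open transforms.
; Door state changes drive sounds and lid light, with some effects gated by a relevance check, and disable focus once open if not closable.
; Door state also supplies the prompt text.
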(event OnDoorStateChanged(BPC_Door)
  (params (DoorState :type EDoorState%20Enum :default "Closed"))
  (CallFunction|HandleDoorStateChange))

(event Custom|OpenCrate
  (bind _newtrack_0 (Timeline|OpenDoor Play)
    (:Update
      (Class|COVDoorComponent|SetDoorStateAlpha (Variables|Default|GetBPC_Door) _newtrack_0))))

(event Custom|CloseCrate
  (bind _newtrack_0 (Timeline|OpenDoor Reverse)
    (:Update
      (Class|COVDoorComponent|SetDoorStateAlpha (Variables|Default|GetBPC_Door) _newtrack_0))))

(event EventBeginPlay
  (bind _bpc_door (Variables|Default|GetBPC_Door))
  (Class|COVDoorComponent|SetDoorHinge _bpc_door (Variables|Default|GetHinge))
  (Class|COVDoorComponent|SetInitialClosedTransform _bpc_door (Transformation|GetRelativeTransform (Variables|Default|GetClosedTransform)))
  (Class|COVDoorComponent|SetFinalOpenTransform _bpc_door (Transformation|GetRelativeTransform (Variables|Default|GetOpenTransform)))
  (CallFunction|SetLights false))

(event Collision|EventActorBeginOverlap
  (params (OtherActor :type Actor%20Object%20Reference)))

(event EventTick
  (params (DeltaSeconds :type Float%20%28single-precision%29)))

(fn ConstructionScript
  (Rendering|SetVisibility (Variables|Default|GetLidLight) false false))

(fn HandleDoorStateChange
  (switch Utilities|FlowControl|Switch|SwitchonEDoorState (Class|COVDoorComponent|GetDoorState (Variables|Default|GetBPC_Door))
    (:Closed
      (Utilities|SwitchEffectsAreRelevant
        (:Relevant
          (CallFunction|SetLights false)
          (CallFunction|PlayClosingEffects))))
    (:Closing
      (CallFunction|CloseCrate)
      (CallFunction|PlaySound "/Game/Audio/PressureValveOpen.PressureValveOpen" 0.8))
    (:Open
      (Utilities|FlowControl|Sequence
        (:then_0
          (if (not (Variables|Default|GetbCanBeClosed))
            (Class|FocusableComponent|SetIsFocusable (Variables|Default|GetFocusable) false)))))
    (:Opening
      (CallFunction|OpenCrate)
      (Utilities|SwitchEffectsAreRelevant
        (:Relevant
          (CallFunction|PlayOpeningEffects)
          (CallFunction|SetLights true))))))

(fn PlayOpeningEffects
  (CallFunction|PlaySound (Variables|Default|GetOpeningSound) 1.0))

(fn CanbeClosed
  (return (Variables|Default|GetbCanBeClosed)))

(fn SetLights
  (params (bEnabled :type Boolean))
  (Rendering|SetVisibility (Variables|Default|GetLidLight) bEnabled bEnabled))

(fn PlayClosingEffects
  (CallFunction|PlaySound (Variables|Default|GetClosingSound) 1.0))

(fn PlaySound
  (params (NewSound :type Sound%20Base%20Object%20Reference) (NewPitchMultiplier :type Float%20%28single-precision%29))
  (bind _audio (Variables|Default|GetAudio))
  (Audio|Components|Audio|SetSound (Variables|Default|GetAudio) NewSound)
  (Audio|Components|Audio|Play _audio 0.0)
  (Audio|Components|Audio|SetPitchMultiplier _audio NewPitchMultiplier))

(fn GetDefaultPromptLocation
  (return (Transformation|GetWorldLocation (Variables|Default|GetPromptLocation))))

(fn GetDefaultPromptText
  (return (Utilities|Select :Index (Class|COVDoorComponent|GetDoorState (Variables|Default|GetBPC_Door)) :Closed "Open" :Closing "Closing..." :Open "Close" :Opening "Opening..." :Locked "Locked")))

(fn GetIsInteractable
  (return (or (Utilities|Enum|Equal(Enum) (Class|COVDoorComponent|GetDoorState (Variables|Default|GetBPC_Door)) "Closed") (Variables|Default|GetbCanBeClosed))))

(fn Interact
  (params (Interactor :type Actor%20Object%20Reference))
  (Utilities|FlowControl|Sequence
    (:then_0
      (switch Utilities|FlowControl|Switch|SwitchonEDoorState (Class|COVDoorComponent|GetDoorState (Variables|Default|GetBPC_Door))
        (:Closed
          (CallFunction|OpenCrate))
        (:Open
          (CallFunction|CloseCrate)))
      (return true))
    (:then_1
      (return false))))