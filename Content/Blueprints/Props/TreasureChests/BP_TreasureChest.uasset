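; BP_TreasureChest is an interactable treasure chest whose lid opens and closes on interaction.
; The construction script configures a BPCDoor component with the lid hinge, deriving the open transform from the closed one by overriding pitch.
; Interact reverses or starts motion based on door state, and the prompt text follows that state.
; The DoorAlpha timeline drives the component's state alpha, playing to open and reversing to close.
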(event Custom|OpenLid
  (bind _dooralpha (Timeline|DoorAlpha Play)
    (:Update
      (Class|COVDoorComponent|SetDoorStateAlpha (Variables|Default|GetBPC_Door) _dooralpha))))

(event Custom|CloseLid
  (bind _dooralpha (Timeline|DoorAlpha Reverse)
    (:Update
      (Class|COVDoorComponent|SetDoorStateAlpha (Variables|Default|GetBPC_Door) _dooralpha))))

(event EventBeginPlay)

(event EventTick
  (params (DeltaSeconds :type Float%20%28single-precision%29)))

(fn ConstructionScript
  (bind _lidhinge (Variables|Default|GetLidHinge))
  (bind _returnvalue (Transformation|GetRelativeTransform _lidhinge))
  (bind (_location _rotation _scale) (Math|Transform|BreakTransform _returnvalue))
  (bind (_roll _pitch _yaw) (Math|Rotator|BreakRotator _rotation))
  (Default|SetDoorHinge (Variables|Default|GetBPC_Door) (Variables|Default|GetLidHinge))
  (Class|COVDoorComponent|SetInitialClosedTransform (Variables|Default|GetBPC_Door) (Transformation|GetRelativeTransform (Variables|Default|GetLidHinge)))
  (Class|COVDoorComponent|SetFinalOpenTransform (Variables|Default|GetBPC_Door) (Math|Transform|MakeTransform _location (Math|Rotator|MakeRotator _roll 1.2e+02 _yaw) _scale)))

(fn GetDefaultPromptLocation
  (return (Transformation|GetWorldLocation (Variables|Default|GetPromptLocation))))

(fn GetDefaultPromptText
  (return (Utilities|Select :Index (Class|COVDoorComponent|GetDoorState (Variables|Default|GetBPC_Door)) :Closed "Open lid" :Closing "Closing..." :Open "Close lid" :Opening "Opening..." :Cracked "Cracked...")))

(fn GetIsInteractable
  (return true))

(fn Interact
  (params (Interactor :type Actor%20Object%20Reference))
  (switch Utilities|FlowControl|Switch|SwitchonEDoorState (Default|GetDoorState (Variables|Default|GetBPC_Door))
    (:Closed
      (CallFunction|OpenLid :!label _label))
    (:Closing
      (goto _label))
    (:Open
      (CallFunction|CloseLid :!label _label_2))
    (:Opening
      (goto _label_2))
    (:Cracked
      (goto _label)))
  (return true))