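; Simple world collectible that offers a "Pick up" interaction prompt and plays a speed-scaled, random-pitch impact sound on hit, throttled by a short gate.
; On authority, Interact spawns the item's inventory actor, adds BPCInventoryItem to the interactor's COVInventory and initializes the spawned actor's COVInventoryItem from it, then destroys the collectible.
; Without a valid actor class it is destroyed without being added; a spawned actor lacking that component prints an error.
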(event Custom|OnMeshHit
  (params (HitComponent :type Primitive%20Component%20Object%20Reference) (OtherActor :type Actor%20Object%20Reference) (OtherComp :type Primitive%20Component%20Object%20Reference) (NormalImpulse :type Vector) (Hit :type Hit%20Result%20Structure%20%28by%20ref%29))
  (bind _returnvalue (Transformation|GetVelocity))
  (bind _returnvalue_2 (Math|Vector|VectorLength _returnvalue))
  (Utilities|FlowControl|Gate false :!label _label
    (:Exit
      (if (>= _returnvalue_2 5e+01)
        (Audio|PlaySoundatLocation "/Game/PrototypeWeap/Sound/Shotgun/Shotgun_BulletImpactB_Cue.Shotgun_BulletImpactB_Cue" (Transformation|GetActorLocation) "0, 0, 0" (* (/ _returnvalue_2 5e+02) 1.0) (Math|Random|RandomFloatinRange 0.8 1.1) 0.0 0 0 0)
        (Utilities|FlowControl|Sequence
          (:then_0
            (goto _label Close))
          (:then_1
            (Utilities|FlowControl|Delay 0.1)
            (goto _label Open)))))))

(event EventBeginPlay
  (Collision|BindEventtoOnComponentHit (Variables|Default|GetCollectibleMesh) (delegate Custom|OnMeshHit)))

(event Collision|EventActorBeginOverlap
  (params (OtherActor :type Actor%20Object%20Reference)))

(event EventTick
  (params (DeltaSeconds :type Float%20%28single-precision%29)))

(fn ConstructionScript)

(fn GetDefaultPromptLocation
  (return (Transformation|GetWorldLocation (Variables|Default|GetInteractPromptTextLocation))))

(fn GetDefaultPromptText
  (return "Pick up"))

(fn GetIsInteractable
  (return true))

(fn Interact
  (params (Interactor :type Actor%20Object%20Reference))
  (bind _bpc_inventoryitem (Variables|Default|GetBPC_InventoryItem))
  (bind _returnvalue (Class|COVInventoryItem|GetCorrespondingItemActorType _bpc_inventoryitem))
  (Networking|SwitchHasAuthority
    (:Authority
      (if (Utilities|IsValidClass _returnvalue)
        (bind _returnvalue_2 (Game|SpawnActorfromClass _returnvalue (Math|Transform|MakeTransform "0, 0, 0" "0, 0, 0" (Transformation|GetWorldScale (Variables|Default|GetCollectibleMesh))) "AlwaysSpawn" 0 0))
        (Class|COVInventory|AddItem (Actor|GetComponentbyClass Interactor "/Script/COV.COVInventory") (Variables|Default|GetBPC_InventoryItem))
        (Utilities|IsValid (Actor|GetComponentbyClass _returnvalue_2 "/Script/COV.COVInventoryItem")
          (:Is%20Valid
            (Class|COVInventoryItem|Initialize (Actor|GetComponentbyClass _returnvalue_2 "/Script/COV.COVInventoryItem") (Variables|Default|GetBPC_InventoryItem)))
          (:Is%20Not%20Valid
            (Development|PrintString (Utilities|String|Append "Error: The spawned inventory version of the item (" (Utilities|GetDisplayName self) ") does not have an inventory item component. Any inventory version of a collectible item needs one.") true true "(R=1.000000,G=0.000000,B=0.000000,A=1.000000)" 11.0)
            (return false))))
      (Actor|DestroyActor)
      (return true))))