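; BP_Crate_A is an interactable sci-fi crate whose lid opens and closes when the player presses F nearby.
; The Box overlap prints a prompt and enables input for player controller 0, and leaving it disables input.
; Each F press flip-flops the Opening timeline forward or in reverse.
; Its Open and MovingUp tracks drive two transform lerps, composed into the Top lid's relative transform.
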(event OnComponentBeginOverlap(Box)
  (params (OverlappedComponent :type Primitive%20Component%20Object%20Reference) (OtherActor :type Actor%20Object%20Reference) (OtherComp :type Primitive%20Component%20Object%20Reference) (OtherBodyIndex :type Integer) (bFromSweep :type Boolean) (SweepResult :type Hit%20Result%20Structure%20%28by%20ref%29))
  ;[1 1 1] player_collider_input
  (Development|PrintString "Press F" true true "(R=0.000000,G=0.660000,B=1.000000,A=1.000000)" 1e+01)
  (Input|EnableInput (Game|GetPlayerController 0)))

(event OnComponentEndOverlap(Box)
  (params (OverlappedComponent :type Primitive%20Component%20Object%20Reference) (OtherActor :type Actor%20Object%20Reference) (OtherComp :type Primitive%20Component%20Object%20Reference) (OtherBodyIndex :type Integer))
  ;[1 1 1] player_collider_input
  (Input|DisableInput (Game|GetPlayerController 0)))

(event Input|KeyboardEvents|F
  (params (Key :type Key%20Structure))
  (:Pressed
    (Utilities|FlowControl|FlipFlop
      (:A
        ;[1 1 1] moving_lid
        (bind (_direction _open _moving_up_) (Timeline|Opening Play)
          (:Update
            (Transformation|SetRelativeTransform (Variables|Default|GetTop) (Math|Transform|ComposeTransforms (Math|Transform|Lerp(Transform) (Variables|Default|Getposition_start) (Variables|Default|Getposition_end) _open) (Math|Transform|Lerp(Transform) (Variables|Default|Getmove_start) (Variables|Default|Getmove_end) _moving_up_)) false false))))
      (:B
        (Timeline|Opening Reverse)))))

(fn ConstructionScript)