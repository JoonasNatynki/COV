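; Interactable double sliding door prop with a rotating lock, front and back text, and a state-based prompt.
; Interacting plays or reverses chained timelines: the lock turns before the doors slide open, and relocks after they close.
; Two door components receive the slide alpha, with closed and open transforms taken from marker components during construction.
; The left door's state drives the prompt, interaction branch, and lock material and point light color.
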(event OnDoorStateChanged(LeftDoor_DoorComponent)
  (params (DoorState :type EDoorState%20Enum :default "Closed"))
  (CallFunction|UpdateLockColor DoorState))

(event Custom|OpenDoor
  ;[1 1 1] Open lock first before opening door
  ;;[1 1 1] Animates the lock
  (bind (_direction _angle) (Timeline|LockAlpha Play)
    (:Update
      (Transformation|SetRelativeRotation (Variables|Default|GetDoorLock) (Math|Rotator|MakeRotator _angle 0.0 0.0) false false))
    (:Finished
      (switch Utilities|FlowControl|Switch|SwitchonETimelineDirection _direction
        (:Forward
          (Variables|Default|SetbIsDoorLockLocked false)
          ;[1 1 1] Close door -> close the lock
          ;;[1 1 1] Animates the door
          (bind (_direction_2 _alpha) (Timeline|DoorAlpha Play)
            (:Update
              (Class|COVDoorComponent|SetDoorStateAlpha (Variables|Default|GetLeftDoor_DoorComponent) _alpha)
              (Class|COVDoorComponent|SetDoorStateAlpha (Variables|Default|GetRightDoor_DoorComponent) _alpha))
            (:Finished
              (switch Utilities|FlowControl|Switch|SwitchonETimelineDirection _direction_2
                (:Backward
                  (Timeline|LockAlpha Reverse))))))
        (:Backward
          (Variables|Default|SetbIsDoorLockLocked true))))))

(event Custom|CloseDoor
  ;[1 1 1] Close door -> close the lock
  ;;[1 1 1] Animates the door
  (bind (_direction _alpha) (Timeline|DoorAlpha Reverse)
    (:Update
      (Class|COVDoorComponent|SetDoorStateAlpha (Variables|Default|GetLeftDoor_DoorComponent) _alpha)
      (Class|COVDoorComponent|SetDoorStateAlpha (Variables|Default|GetRightDoor_DoorComponent) _alpha))
    (:Finished
      (switch Utilities|FlowControl|Switch|SwitchonETimelineDirection _direction
        (:Backward
          ;[1 1 1] Open lock first before opening door
          ;;[1 1 1] Animates the lock
          (bind (_direction_2 _angle) (Timeline|LockAlpha Reverse)
            (:Update
              (Transformation|SetRelativeRotation (Variables|Default|GetDoorLock) (Math|Rotator|MakeRotator _angle 0.0 0.0) false false))
            (:Finished
              (switch Utilities|FlowControl|Switch|SwitchonETimelineDirection _direction_2
                (:Forward
                  (Variables|Default|SetbIsDoorLockLocked false)
                  (Timeline|DoorAlpha Play))
                (:Backward
                  (Variables|Default|SetbIsDoorLockLocked true))))))))))

(event EventBeginPlay)

(event Collision|EventActorBeginOverlap
  (params (OtherActor :type Actor%20Object%20Reference)))

(event EventTick
  (params (DeltaSeconds :type Float%20%28single-precision%29)))

(fn ConstructionScript
  (Utilities|FlowControl|Sequence
    (:then_0
      ;[1 1 1] Initialize door hinges
      (Default|SetDoorHinge (Variables|Default|GetLeftDoor_DoorComponent) (Variables|Default|GetLeftDoorHinge))
      (Default|SetDoorHinge (Variables|Default|GetRightDoor_DoorComponent) (Variables|Default|GetRightDoorHinge)))
    (:then_1
      (Class|COVDoorComponent|SetInitialClosedTransform (Variables|Default|GetLeftDoor_DoorComponent) (Transformation|GetRelativeTransform (Variables|Default|GetClosedPositionLeft)))
      (Class|COVDoorComponent|SetInitialClosedTransform (Variables|Default|GetRightDoor_DoorComponent) (Transformation|GetRelativeTransform (Variables|Default|GetClosedPositionRight)))
      (Class|COVDoorComponent|SetFinalOpenTransform (Variables|Default|GetLeftDoor_DoorComponent) (Transformation|GetRelativeTransform (Variables|Default|GetOpenPositionLeft)))
      (Class|COVDoorComponent|SetFinalOpenTransform (Variables|Default|GetRightDoor_DoorComponent) (Transformation|GetRelativeTransform (Variables|Default|GetOpenPositionRight))))
    (:then_2
      (bind _returnvalue (Rendering|Material|CreateDynamicMaterialInstance (Variables|Default|GetDoorLock) 0 "/Game/Blueprints/Props/Doors/Materials/M_UE4_Logo_Door.M_UE4_Logo_Door" "None" :!class /Script/Engine.PrimitiveComponent))
      (Variables|Default|SetLockMaterial _returnvalue))
    (:then_3
      (CallFunction|UpdateLockColor (Class|COVDoorComponent|GetDoorState (Variables|Default|GetLeftDoor_DoorComponent))))
    (:then_4
      (Rendering|Components|TextRender|SetText (Variables|Default|GetBackText) (Variables|Default|GetBackTextText))
      (Rendering|Components|TextRender|SetText (Variables|Default|GetFrontText) (Variables|Default|GetFrontTextText)))))

(fn UpdateLockColor
  (params (Index :type EDoorState%20Enum :default "Closed"))
  (bind _returnvalue (Utilities|Select :Index Index :Closed "(R=1.000000,G=0.009271,B=0.000000,A=1.000000)" :Closing "(R=0.270833,G=0.000000,B=0.000000,A=1.000000)" :Open "(R=0.000000,G=0.989583,B=0.014296,A=1.000000)" :Opening "(R=0.000000,G=0.177083,B=0.000000,A=1.000000)" :Locked ""))
  (Rendering|Material|SetVectorParameterValue (Variables|Default|GetLockMaterial) "Color" _returnvalue :!class /Script/Engine.MaterialInstanceDynamic)
  (Rendering|Components|Light|SetLightColor (Variables|Default|GetPointLight) _returnvalue true))

(fn OnRepBIsDoorLockLocked)

(fn GetDefaultPromptLocation
  (return (Transformation|GetWorldLocation (Variables|Default|GetPromptLocation))))

(fn GetDefaultPromptText
  (return (Utilities|Select :Index (Class|COVDoorComponent|GetDoorState (Variables|Default|GetLeftDoor_DoorComponent)) :Closed "Open door" :Closing "Closing..." :Open "Close door" :Opening "Opening..." :Locked "")))

(fn GetIsInteractable
  (return true))

(fn Interact
  (params (Interactor :type Actor%20Object%20Reference))
  (switch Utilities|FlowControl|Switch|SwitchonEDoorState (Default|GetDoorState (Variables|Default|GetLeftDoor_DoorComponent))
    (:Closed
      (CallFunction|OpenDoor :!label _label))
    (:Closing
      (goto _label))
    (:Open
      (CallFunction|CloseDoor :!label _label_2))
    (:Opening
      (goto _label_2)))
  (return true))