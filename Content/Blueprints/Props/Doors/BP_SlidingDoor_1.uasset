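; Interactable sliding door prop that opens or closes on interaction, with prompt text that follows the door's state.
; The construction script passes the hinge and closed/open transforms to the BPCDoor component.
; Interact picks open or close from that state through server events, which play or reverse a timeline that drives the component's door alpha.
; The prompt location returns zero, leaving the InteractionPromptLocation component's position unused.
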(event Custom|OpenDoor_Server
  (bind _doorstatealpha (Timeline|Timeline_0 Play)
    (:Update
      (Class|COVDoorComponent|SetDoorStateAlpha (Variables|Default|GetBPC_Door) _doorstatealpha))))

(event Custom|CloseDoor_Server
  (bind _doorstatealpha (Timeline|Timeline_0 Reverse)
    (:Update
      (Class|COVDoorComponent|SetDoorStateAlpha (Variables|Default|GetBPC_Door) _doorstatealpha))))

(event EventBeginPlay)

(event Collision|EventActorBeginOverlap
  (params (OtherActor :type Actor%20Object%20Reference)))

(event EventTick
  (params (DeltaSeconds :type Float%20%28single-precision%29)))

(fn ConstructionScript
  (Default|SetDoorHinge (Variables|Default|GetBPC_Door) (Variables|Default|GetDoorHinge))
  (Class|COVDoorComponent|SetInitialClosedTransform (Variables|Default|GetBPC_Door) (Transformation|GetRelativeTransform (Variables|Default|GetClosedTransform)))
  (Class|COVDoorComponent|SetFinalOpenTransform (Variables|Default|GetBPC_Door) (Transformation|GetRelativeTransform (Variables|Default|GetOpenTransform))))

(fn GetDefaultPromptLocation
  (return "0, 0, 0"))

(fn GetDefaultPromptText
  (return (Utilities|Select :Index (Default|GetDoorState (Variables|Default|GetBPC_Door)) :Closed "Open door" :Closing "Closing..." :Open "Close door" :Opening "Opening..." :Cracked "Cracked...")))

(fn GetIsInteractable
  (return true))

(fn Interact
  (params (Interactor :type Actor%20Object%20Reference))
  (if (Utilities|Select :Index (Class|COVDoorComponent|GetDoorState (Variables|Default|GetBPC_Door)) :Closed true :Closing true :Open false :Opening false :Cracked true)
    (CallFunction|OpenDoorServer)
    (else
      (CallFunction|CloseDoorServer)))
  (return true))