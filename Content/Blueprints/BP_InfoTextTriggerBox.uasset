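; BP_InfoTextTriggerBox is a trigger volume that shows an info text screen when a Character enters it.
; On overlap, where effects are relevant, it pushes WBP_InfoScreen to that character's player controller with the configured InfoData and lifetime.
; A valid screen sets InfoAlreadyDisplayedOnce, which gates one-shot display.
; As written, Repeatable boxes display only if that flag is already true, so they never fire from a false start.
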(event OnComponentBeginOverlap(CollisionComponent)
  (params (OverlappedComponent :type Primitive%20Component%20Object%20Reference) (OtherActor :type Actor%20Object%20Reference) (OtherComp :type Primitive%20Component%20Object%20Reference) (OtherBodyIndex :type Integer) (bFromSweep :type Boolean) (SweepResult :type Hit%20Result%20Structure%20%28by%20ref%29))
  (if (CallFunction|CanInfobeDisplayedStill)
    (bind _ascharacter (Utilities|Casting|CastToCharacter OtherActor)) ; Only characters need info texts
    (Utilities|SwitchEffectsAreRelevant
      (:Relevant
        (bind _returnvalue (|PushScreenbyClass "/Game/UI/Widgets/Screens/Info/WBP_InfoScreen.WBP_InfoScreen_C" (.AsPlayer%20Controller (Utilities|Casting|CastToPlayerController (Pawn|GetController _ascharacter))) (Variables|Default|GetInfoData) (Variables|Default|GetInfoLifeTime)))
        (Utilities|IsValid _returnvalue
          (:Is%20Valid
            (Variables|Internal|SetbInfoAlreadyDisplayedOnce true)))))))

(event EventBeginPlay)

(event Collision|EventActorBeginOverlap
  (params (OtherActor :type Actor%20Object%20Reference)))

(event EventTick
  (params (DeltaSeconds :type Float%20%28single-precision%29)))

(fn ConstructionScript)

(fn CanInfobeDisplayedStill
  (return (or (and (not (Variables|Default|GetbRepeatable)) (not (Variables|Internal|GetbInfoAlreadyDisplayedOnce))) (and (Variables|Default|GetbRepeatable) (Variables|Internal|GetbInfoAlreadyDisplayedOnce)))))