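; A collectible item actor that can be picked up into the interacting actor's InventoryComponent.
; Its construction script hands the static mesh to a HoveringMotion component as the component to hover.
; Interaction functions report it as always interactable, with a "Pick up" prompt at the actor's location.
; Interact adds the item itself to the inventory only with authority, returning that result, and returns false on remote.
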(event EventBeginPlay)

(event Collision|EventActorBeginOverlap
  (params (OtherActor :type Actor%20Object%20Reference)))

(event EventTick
  (params (DeltaSeconds :type Float%20%28single-precision%29)))

(fn ConstructionScript
  (Class|HoveringMotion|SetHoveringComponent (Variables|Default|GetHoveringMotion) (Variables|Default|GetStaticMesh)))

(fn GetDefaultPromptLocation
  (return (Transformation|GetActorLocation)))

(fn GetDefaultPromptText
  (return "Pick up"))

(fn GetIsInteractable
  (return true))

(fn Interact
  (params (Interactor :type Actor%20Object%20Reference))
  (Networking|SwitchHasAuthority
    (:Authority
      (bind _returnvalue (Class|InventoryComponent|AddItem (Actor|GetComponentbyClass Interactor "/Script/InventoryAndItems.InventoryComponent") self))
      (return _returnvalue))
    (:Remote
      (return false))))