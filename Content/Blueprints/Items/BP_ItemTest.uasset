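; BP_ItemTest is a test item that an interactor can add to its inventory.
; It implements interaction functions, always reporting itself interactable and supplying a hard-coded placeholder prompt, crude in wording, at the PromptTextLocation component's world position.
; Interact passes BPCInventoryItem to AddItem on the interactor's BPC_Inventory component and returns true, without checking that the component exists or removing the item actor.
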(event EventBeginPlay)

(event Collision|EventActorBeginOverlap
  (params (OtherActor :type Actor%20Object%20Reference)))

(event EventTick
  (params (DeltaSeconds :type Float%20%28single-precision%29)))

(fn ConstructionScript)

(fn GetDefaultPromptLocation
  (return (Transformation|GetWorldLocation (Variables|Default|GetPromptTextLocation))))

(fn GetDefaultPromptText
  (return "Touch my tits!"))

(fn GetIsInteractable
  (return true))

(fn Interact
  (params (Interactor :type Actor%20Object%20Reference))
  (Class|COVInventory|AddItem (Actor|GetComponentbyClass Interactor "/Game/Blueprints/Components/BPC_Inventory.BPC_Inventory_C") (Variables|Default|GetBPC_InventoryItem))
  (return true))