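; BP_COVPlayerController is a player controller that handles debug and screen-stack input and can request actor spawns on the server.
; F6 shows the debug window through the HUD only when no WBP_DebugMenu screen exists, and Escape pops the top screen, both where effects are relevant.
; Server_SpawnActor, on authority, forwards the spawn to the Development game mode with itself as owner.
; The left mouse handler is empty, and a camera-ray debug line is left unconnected.
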(event Custom|Server_SpawnActor
  (params (SpawnTransform :type Transform) (CollisionHandlingOverride :type ESpawnActorCollisionHandlingMethod%20Enum :default "Undefined") (Class :type Actor%20Class%20Reference))
  ;[1 0.2188 0.826] Make better
  (Networking|SwitchHasAuthority
    (:Authority
      (Default|SpawnActor (.AsDevelopment (Utilities|Casting|CastToDevelopment (Game|GetGameMode))) SpawnTransform CollisionHandlingOverride self Class))))

(event EventBeginPlay
  (|CallParentFunction))

(event EventTick
  (params (DeltaSeconds :type Float%20%28single-precision%29))
  (|CallParentFunction DeltaSeconds))

(event EventInputLeftMouseButtonPressed)

(event Input|KeyboardEvents|F6
  (params (Key :type Key%20Structure :default "None"))
  (:Pressed
    (Utilities|SwitchEffectsAreRelevant
      (:Relevant
        (bind _screensfound (Class|ICOVHUD|FindScreensOfType(Message) (HUD|GetHUD) "/Game/UI/Widgets/Screens/WBP_DebugMenu.WBP_DebugMenu_C"))
        (Class|ICOVHUD|SetDebugWindowActive(Message) (HUD|GetHUD) (Class|E4CodeHelpers|IsArrayEmpty _screensfound))))))

(event Input|KeyboardEvents|Escape
  (params (Key :type Key%20Structure :default "None"))
  (:Pressed
    (Utilities|SwitchEffectsAreRelevant
      (:Relevant
        (bind _screenstack (Class|ICOVHUD|GetScreenStack(Message) (HUD|GetHUD)))
        (Class|ScreenStack|PopTopScreen _screenstack)))))

(fn ConstructionScript)