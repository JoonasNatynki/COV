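; Component that adapts reverb to the surroundings of its owning actor.
; Tick uses a 0.2-second Delay to throttle echo profile generation from the owner's skeletal mesh Head socket, then activates a reverb effect with a fade.
; Squared echo coverage times the float profile picks a reverb preset through nested thresholds, while squared coverage alone, scaled and clamped, sets the volume.
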(event EventBeginPlay)

(event EventTick
  (params (DeltaSeconds :type Float%20%28single-precision%29))
  (Utilities|FlowControl|Delay 0.2)
  (Class|COVEchoProfiler|GenerateEchoProfile (Transformation|GetSocketLocation (Actor|GetComponentbyClass (Components|GetOwner) "/Script/Engine.SkeletalMeshComponent") "Head"))
  (Class|GameplayStatics|ActivateReverbEffect (CallFunction|GetReverbProfilefromEchoProfile) "EchoProfile" 1.0 (CallFunction|GetReverbVolume) 1.0))

(fn GetCustomEchoProfile
  (return (* (Math|Float|Power (Class|COVEchoProfiler|GetEchoCoverageProfile) 2.0) (Class|COVEchoProfiler|GetEchoFloatProfile))))

(fn GetReverbProfilefromEchoProfile
  (bind _returnvalue (CallFunction|GetCustomEchoProfile))
  (return (select (> _returnvalue 1e+01) (select (> _returnvalue 3e+01) (select (> _returnvalue 5e+01) (select (> _returnvalue 7e+01) (select (> _returnvalue 1e+02) "/Engine/EngineSounds/ReverbSettings/CaveHall.CaveHall" "/Engine/EngineSounds/ReverbSettings/StoneRoom.StoneRoom") "/Engine/EngineSounds/ReverbSettings/ConcertHall.ConcertHall") "/Engine/EngineSounds/ReverbSettings/Cave.Cave") (select (> _returnvalue 2e+01) "/Engine/EngineSounds/ReverbSettings/Alley.Alley" "/Engine/EngineSounds/ReverbSettings/Bathroom.Bathroom")) (select (> _returnvalue 2.5) "/Engine/EngineSounds/ReverbSettings/LargeRoom.LargeRoom" "/Engine/EngineSounds/ReverbSettings/Underwater.Underwater"))))

(fn GetReverbVolume
  (return (Math|Float|Clamp(Float) (* (Math|Float|Power (Class|COVEchoProfiler|GetEchoCoverageProfile) 2.0) 2.5))))