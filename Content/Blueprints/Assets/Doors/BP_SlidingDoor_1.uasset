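; Interactable sliding door that opens or closes on interaction and shows prompt text based on its current state.
; The construction script passes the DoorHinge and the relative open and closed marker transforms to the BPCDoor component.
; Interact picks the open or close server event from the door state; opening plays a timeline that feeds BPCDoor's state alpha, and closing reverses it.
; The default prompt location returns a zero vector, leaving InteractionPromptLocation unused.
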(event Custom|OpenDoor_Server
  (bind _doorstatealpha (Timeline|Timeline_0 Play)
    (:Update
      (Default|SetDoorStateAlpha (Variables|Default|GetBPC_Door) _doorstatealpha))))

(event Custom|CloseDoor_Server
  (bind _doorstatealpha (Timeline|Timeline_0 Reverse)
    (:Update
      (Default|SetDoorStateAlpha (Variables|Default|GetBPC_Door) _doorstatealpha))))

(event EventBeginPlay)

(event Collision|EventActorBeginOverlap
  (params (OtherActor :type Actor%20Object%20Reference)))

(event EventTick
  (params (DeltaSeconds :type Float%20%28single-precision%29)))

(fn ConstructionScript
  (Default|SetDoorHinge (Variables|Default|GetBPC_Door) (Variables|Default|GetDoorHinge))
  (Variables|/Game/Blueprints/Assets/Doors/BPC_Door.BPC_Door_C|SetInitialClosedTransformation (Variables|Default|GetBPC_Door) (Transformation|GetRelativeTransform (Variables|Default|GetClosedTransform)))
  (Variables|/Game/Blueprints/Assets/Doors/BPC_Door.BPC_Door_C|SetFinalOpenTransformation (Variables|Default|GetBPC_Door) (Transformation|GetRelativeTransform (Variables|Default|GetOpenTransform))))

(fn GetDefaultPromptLocation
  (return "0, 0, 0"))

(fn GetDefaultPromptText
  (return (Utilities|Select :Index (Default|GetDoorState (Variables|Default|GetBPC_Door)) :NewEnumerator0 "Open door" :NewEnumerator2 "" :NewEnumerator1 "Close door" :NewEnumerator3 "" :NewEnumerator4 "Open door")))

(fn GetIsInteractable
  (return true))

(fn Interact
  (params (Interactor :type Actor%20Object%20Reference))
  (if (Utilities|Select :Index (Default|GetDoorState (Variables|Default|GetBPC_Door)) :NewEnumerator0 true :NewEnumerator2 true :NewEnumerator1 false :NewEnumerator3 false :NewEnumerator4 true)
    (CallFunction|OpenDoorServer)
    (else
      (CallFunction|CloseDoorServer)))
  (return true))