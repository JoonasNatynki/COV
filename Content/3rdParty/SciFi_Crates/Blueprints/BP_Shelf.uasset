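; BP_Shelf is a modular shelving actor that builds a grid of racks from depth, length and height levels.
; Its construction script places instanced support beams, bases, platforms and shelf parts at fixed spacing, using division and modulo to derive grid positions.
; The platform loop is nested inside the support loop, so platforms, shelf parts and, on taller racks, bases receive overlapping duplicate instances.
; The event graph is empty.
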(event EventBeginPlay)

(event Collision|EventActorBeginOverlap
  (params (OtherActor :type Actor%20Object%20Reference)))

(event EventTick
  (params (DeltaSeconds :type Float%20%28single-precision%29)))

(fn ConstructionScript
  (bind _shelf_height_level (Variables|Default|GetSHelf%20Height%20Level))
  (bind _support_beams_array (Variables|Default|GetSupport%20Beams%20Array))
  (bind _shelf_height_level_2 (Variables|Default|GetSHelf%20Height%20Level))
  (bind _shelf_platform_array (Variables|Default|GetShelf%20Platform%20Array))
  (bind _returnvalue (+ _shelf_height_level_2 -1))
  ;[1 1 1] Creating XYZ Array for Support Beams
  (Utilities|Array|Resize _support_beams_array (Variables|Default|GetShelf%20Depth%20Level))
  (for (_ _array_index) _support_beams_array
    (for _index (range 0 (- (* (Variables|Default|GetShelf%20Length%20Level) _returnvalue) 1))
      ;[1 1 1] Placement Support Beams Instances
      (Components|InstancedStaticMesh|AddInstance (Variables|Default|GetSupport) (Math|Transform|MakeTransform (Math|Vector|MakeVector (* _array_index 2e+02) (* (/ _index _returnvalue) 2e+02) (* (Math|Integer|%(Integer) _index _returnvalue) 1.2e+02))))
      (Components|InstancedStaticMesh|AddInstance (Variables|Default|GetSupport_Base) (Math|Transform|MakeTransform (Math|Vector|MakeVector (* _array_index 2e+02) (* (/ _index _returnvalue) 2e+02) 0.0)))
      ;[1 1 1] Creating XYZ Array for Shelf Platform
      (Utilities|Array|Resize _shelf_platform_array (- (Variables|Default|GetShelf%20Depth%20Level) 1))
      (for (_ _array_index_2) _shelf_platform_array
        (for _index_2 (range 0 (- (* (- (Variables|Default|GetShelf%20Length%20Level) 1) (Variables|Default|GetSHelf%20Height%20Level)) 1))
          ;[1 1 1] Placement Shelf Platform Instances
          (Components|InstancedStaticMesh|AddInstance (Variables|Default|GetShelf) (Math|Transform|MakeTransform (Math|Vector|MakeVector (* _array_index_2 2e+02) (* (/ _index_2 _shelf_height_level) 2e+02) (* (Math|Integer|%(Integer) _index_2 _shelf_height_level) 1.2e+02))))
          (Components|InstancedStaticMesh|AddInstance (Variables|Default|GetShelf_Part) (Math|Transform|MakeTransform (Math|Vector|MakeVector (* _array_index 2e+02) (* (/ _index_2 _shelf_height_level) 2e+02) (* (Math|Integer|%(Integer) _index_2 _shelf_height_level) 1.2e+02)))))))))