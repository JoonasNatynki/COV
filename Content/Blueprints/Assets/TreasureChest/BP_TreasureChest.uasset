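; Treasure chest Blueprint with a hinged lid that opens and closes on interaction.
; A door component (BPCDoor) takes the lid hinge in the construction script and tracks the lid state, while the DoorAlpha timeline drives its alpha forward or in reverse.
; Interact toggles by that state and can reverse mid-motion.
; The same state selects the prompt text, shown at a dedicated prompt location.
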(event Custom|OpenLid
  (bind _dooralpha (Timeline|DoorAlpha Play)
    (:Update
      (Default|SetDoorStateAlpha (Variables|Default|GetBPC_Door) _dooralpha))))

(event Custom|CloseLid
  (bind _dooralpha (Timeline|DoorAlpha Reverse)
    (:Update
      (Default|SetDoorStateAlpha (Variables|Default|GetBPC_Door) _dooralpha))))

(event EventBeginPlay)

(event EventTick
  (params (DeltaSeconds :type Float%20%28single-precision%29)))

(fn ConstructionScript
  (Default|SetDoorHinge (Variables|Default|GetBPC_Door) (Variables|Default|GetLidHinge)))

(fn GetDefaultPromptLocation
  (return (Transformation|GetWorldLocation (Variables|Default|GetPromptLocation))))

(fn GetDefaultPromptText
  (return (Utilities|Select :Index (Default|GetDoorState (Variables|Default|GetBPC_Door)) :NewEnumerator0 "Open lid" :NewEnumerator2 "Closing..." :NewEnumerator1 "Close lid" :NewEnumerator3 "Opening..." :NewEnumerator4 "Open lid")))

(fn GetIsInteractable
  (return true))

(fn Interact
  (params (Interactor :type Actor%20Object%20Reference))
  (switch Utilities|FlowControl|Switch|SwitchonE_DoorState (Default|GetDoorState (Variables|Default|GetBPC_Door))
    (:NewEnumerator0
      (CallFunction|OpenLid :!label _label))
    (:NewEnumerator2
      (goto _label))
    (:NewEnumerator1
      (CallFunction|CloseLid :!label _label_2))
    (:NewEnumerator3
      (goto _label_2))
    (:NewEnumerator4
      (goto _label)))
  (return true))