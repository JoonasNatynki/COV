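; BP_COVCharacter is a character pawn with echo profiling, an inspection close-up camera and an inventory component.
; Tick, throttled by a 0.2-second Delay, has EchoProfiler generate an echo profile from the mesh's Head socket location.
; Pressing E alternately plays and reverses a timeline that drives spring arm length for the close-up.
; The inventory change handler is empty, and a delayed remove-on-add branch is left disconnected.
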(event OnInventoryChanged(BPC_Inventory)
  (params (_action :type Inventory%20Action%20Structure%20%28by%20ref%29)))

(event EventBeginPlay)

(event Collision|EventActorBeginOverlap
  (params (OtherActor :type Actor%20Object%20Reference)))

(event EventInputEPressed
  ;[1 1 1] Closeup camera
  (Utilities|FlowControl|FlipFlop
    (:A
      (bind _springarmlengthmultiplier (Timeline|InspectionCameraMode Play)
        (:Update
          (Variables|/Script/Engine.SpringArmComponent|SetTargetArmLength (Variables|Default|GetSpringArm) _springarmlengthmultiplier))))
    (:B
      (Timeline|InspectionCameraMode Reverse))))

(event EventTick
  (params (DeltaSeconds :type Float%20%28single-precision%29))
  (Utilities|FlowControl|Delay 0.2)
  (Class|EchoProfiler|GenerateEchoProfile (Variables|Default|GetEchoProfiler) (Transformation|GetSocketLocation (Variables|Character|GetMesh) "Head")))

(fn ConstructionScript)