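; BP_ItemTest_Collectible is a test collectible item that an interactor can pick up into its inventory.
; It always reports itself interactable and supplies a hard-coded placeholder prompt, positioned at its PromptTextLocation component.
; Interact adds BPCInventoryItem to the interactor's BPC_Inventory and returns true, or prints a warning when that component is missing.
; The actor is never hidden or destroyed here, and its event graph is empty.
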(event EventBeginPlay)

(event Collision|EventActorBeginOverlap
  (params (OtherActor :type Actor%20Object%20Reference)))

(event EventTick
  (params (DeltaSeconds :type Float%20%28single-precision%29)))

(fn ConstructionScript)

(fn GetDefaultPromptLocation
  (return (Transformation|GetWorldLocation (Variables|Default|GetPromptTextLocation))))

(fn GetDefaultPromptText
  (return "Touch my tits!"))

(fn GetIsInteractable
  (return true))

(fn Interact
  (params (Interactor :type Actor%20Object%20Reference))
  (bind _returnvalue (Actor|GetComponentbyClass Interactor "/Game/Blueprints/Components/BPC_Inventory.BPC_Inventory_C"))
  (Utilities|IsValid _returnvalue
    (:Is%20Valid
      (Class|COVInventory|AddItem _returnvalue (Variables|Default|GetBPC_InventoryItem))
      (return true))
    (:Is%20Not%20Valid
      (Development|PrintString "Warning: Item will not interact with the interactor: No inventory found on the interactor" false))))