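; Replicated treasure chest actor that opens its lid when an actor begins overlapping it and closes it when an overlap ends.
; Only the authority changes the Open flag, and its RepNotify calls OpenLid or CloseLid.
; These events play or reverse the OpenTreasureChest timeline, whose Angle track drives the pitch of the LidHinge component.
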(event Custom|OpenLid
  (bind _angle (Timeline|OpenTreasureChest Play)
    (:Update
      (Transformation|SetRelativeRotation (Variables|Default|GetLidHinge) (Math|Rotator|MakeRotator 0.0 _angle 0.0) false false))))

(event Custom|CloseLid
  (bind _angle (Timeline|OpenTreasureChest Reverse)
    (:Update
      (Transformation|SetRelativeRotation (Variables|Default|GetLidHinge) (Math|Rotator|MakeRotator 0.0 _angle 0.0) false false))))

(event EventBeginPlay)

(event Collision|EventActorBeginOverlap
  (params (OtherActor :type Actor%20Object%20Reference))
  (Networking|SwitchHasAuthority
    (:Authority
      (Variables|Default|SetbOpen true))))

(event EventTick
  (params (DeltaSeconds :type Float%20%28single-precision%29)))

(event Collision|EventActorEndOverlap
  (params (OtherActor :type Actor%20Object%20Reference))
  (Networking|SwitchHasAuthority
    (:Authority
      (Variables|Default|SetbOpen false))))

(fn ConstructionScript)

(fn OnRepBOpen
  (if (Variables|Default|GetbOpen)
    (CallFunction|OpenLid)
    (else
      (CallFunction|CloseLid))))