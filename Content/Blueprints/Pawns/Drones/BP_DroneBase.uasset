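; Base flying drone with player controls for vertical movement and turbo speed, plus server-driven movement along a spline.
; Tick steers the authority copy toward a time-based spline point and uses gates to fire stopped and start-moving dispatchers, whose local handlers are empty.
; Where effects are relevant, a timeline animates hovering and engine pitch follows velocity.
; Construction initializes lights, with one intensity value driving point light and material glow.
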(event Custom|OnStopped_Event)

(event Custom|OnStartMoving_Event)

(event EventBeginPlay
  (Components|Timeline|SetPlayRate (Variables|Default|GetStationaryHoverAnimation) 0.12)
  (Utilities|FlowControl|Sequence
    (:then_0
      (Utilities|SwitchEffectsAreRelevant
        (:Relevant
          (bind _offsetmultiplier (Timeline|StationaryHoverAnimation Play)
            (:Update
              (Transformation|SetRelativeLocation (Variables|Default|GetStaticMesh) (Math|Vector|MakeVector 0.0 0.0 (* _offsetmultiplier 18.0)) false false)
              (Transformation|AddLocalRotation (Variables|Default|GetStaticMesh) "0.200000,0.200000, 0" false false))))))
    (:then_1
      (EventDispatchers|BindEventtoOnStopped (delegate Custom|OnStopped_Event)))
    (:then_2
      (EventDispatchers|BindEventtoOnStartMoving (delegate Custom|OnStartMoving_Event)))
    (:then_3
      (Utilities|SwitchEffectsAreRelevant
        (:Relevant
          (Audio|Components|Audio|Play (Variables|Default|GetEngine) 0.0))))
    (:then_4
      (Utilities|SwitchEffectsAreRelevant
        (:Relevant
          (Transformation|SetRelativeRotation (Variables|Default|GetStaticMesh) (Math|Random|RandomRotator true) false false))))
    (:then_6
      (Networking|SwitchHasAuthority))))

(event Collision|EventActorBeginOverlap
  (params (OtherActor :type Actor%20Object%20Reference)))

(event EventTick
  (params (DeltaSeconds :type Float%20%28single-precision%29))
  (bind _actorwithspline (Variables|Default|GetActorWithSpline))
  (bind _returnvalue (Actor|GetComponentbyClass _actorwithspline "/Script/Engine.SplineComponent"))
  (Utilities|FlowControl|Sequence
    (:then_0
      ;[0 0.02083 0.002165] Update and call OnStopped/OnStartMoving when they happen
      (if (CallFunction|IsStationary)
        (Utilities|FlowControl|Gate false :!label _label
          (:Exit
            (Default|CallOnStopped)
            (Utilities|FlowControl|Sequence
              (:then_0
                (goto _label_2 Open))
              (:then_1
                (goto _label Close)))))
        (else
          (Utilities|FlowControl|Gate false :!label _label_2
            (:Exit
              (Default|CallOnStartMoving)
              (Utilities|FlowControl|Sequence
                (:then_0
                  (goto _label Open))
                (:then_1
                  (goto _label_2 Close))))))))
    (:then_1
      (Utilities|SwitchEffectsAreRelevant
        (:Relevant
          (Utilities|FlowControl|Sequence
            (:then_0
              (Updates|UpdateEnginePitch))
            (:then_1
              (Updates|UpdateMovingUpInput))
            (:then_2
              (Updates|UpdateMovingDownInput))))))
    (:then_2
      (Networking|SwitchHasAuthority
        (:Authority
          (Pawn|Input|AddMovementInput (- (Spline|GetLocationatDistanceAlongSpline _returnvalue (Math|Float|%(Float) (* (Actor|GetGameTimeSinceCreation) 1e+02) (Spline|GetSplineLength _returnvalue)) "World") (Transformation|GetActorLocation)) 0.005 false))))))

(event Custom|Server_SetMaxFlySpeed
  (params (MaxFlySpeed :type Float%20%28single-precision%29))
  (Variables|/Script/Engine.CharacterMovementComponent|SetMaxFlySpeed (Variables|Character|GetCharacterMovement) MaxFlySpeed))

(event EventInputLeftControlPressed
  (Variables|Internal|SetbLControlPressed true))

(event EventInputLeftControlReleased
  (Variables|Internal|SetbLControlPressed false))

(event EventInputLeftShiftPressed
  (CallFunction|ServerSetMaxFlySpeed (Variables|Default|GetDroneTurboFlyingSpeed)))

(event EventInputLeftShiftReleased
  (CallFunction|ServerSetMaxFlySpeed (Variables|Default|GetDroneDefaultFlyingSpeed)))

(event EventInputSpacebarPressed
  (Variables|Internal|SetbSpaceBarPressed true))

(event EventInputSpacebarReleased
  (Variables|Internal|SetbSpaceBarPressed false))

(fn ConstructionScript
  (CallFunction|InitializeLights))

(fn IsStationary
  (return (== (Math|Vector|VectorLength (Variables|/Script/Engine.MovementComponent|GetVelocity (Variables|Character|GetCharacterMovement))) 0.0)))

(fn SetLightIntensity
  (params (LightIntensity :type Float%20%28single-precision%29))
  (Variables|Default|SetLightsIntensity LightIntensity)
  (Rendering|Components|Light|SetIntensity (Variables|Default|GetPointLight) (* (Variables|Internal|GetLightDefaultIntensity) (Math|Float|Power (Variables|Default|GetLightsIntensity) 3.0)))
  (Rendering|Material|SetVectorParameterValueonMaterials (Variables|Default|GetStaticMesh) "GlowColor" (Math|Conversions|ToVector(LinearColor) (* (Variables|Default|GetLightColors) (* (Variables|Default|GetLightsIntensity) 1e+02))))
  (Rendering|Components|Light|SetLightColor (Variables|Default|GetPointLight) (Variables|Default|GetLightColors) true))

(fn UpdateEnginePitch
  (Audio|Components|Audio|SetPitchMultiplier (Variables|Default|GetEngine) (Math|Float|MapRangeClamped (Math|Vector|VectorLength (Variables|/Script/Engine.MovementComponent|GetVelocity (Variables|Character|GetCharacterMovement))) 0.0 (Variables|Default|GetDroneTurboFlyingSpeed) 0.5 2.0)))

(fn InitializeLights
  (Variables|Internal|SetLightDefaultIntensity (Variables|/Script/Engine.LightComponentBase|GetIntensity (Variables|Default|GetPointLight)))
  (CallFunction|SetLightIntensity (Variables|Default|GetLightsIntensity)))

(fn UpdateMovingUpInput
  (if (Variables|Internal|GetbSpaceBarPressed)
    (Class|PawnMovementComponent|AddInputVector (Variables|Character|GetCharacterMovement) (* (Transformation|GetActorUpVector) 1.0) false)))

(fn UpdateMovingDownInput
  (if (Variables|Internal|GetbLControlPressed)
    (Class|PawnMovementComponent|AddInputVector (Variables|Character|GetCharacterMovement) (* (Transformation|GetActorUpVector) -1.0) false)))

(fn Interact
  (params (Interactor :type Actor%20Object%20Reference))
  (return false))

(fn SetLightColors)